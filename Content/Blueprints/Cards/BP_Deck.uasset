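; BP_Deck is a playing card deck actor with Texas Hold'em-style dealing functions.
; On BeginPlay it builds 52 card structs from suit and rank, matching textures by a T_Suit_Rank name, then shuffles a copy using Fisher-Yates.
; Deal functions pull cards from the top of the shuffled array, though DealFlop returns nothing and DealTurn and DealRiver are empty stubs.
; Two debug events print either deck to screen.
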(event Custom|PrintDeckToScreen
  ;[0.15 0.1397 0.002652 0.5] Deck/Shuffle testing
  (for (_ _array_index) (Variables|Default|GetDeck)
    (Development|PrintString (Utilities|String|ToString(Text) (Utilities|Text|FormatText "Suit = {Suit}, Rank = {Rank}, Texture {Texture}" (Utilities|String|EnumtoString (.suit (Utilities|Array|Get(acopy) (Variables|Default|GetDeck) _array_index))) (.rank (Utilities|Array|Get(acopy) (Variables|Default|GetDeck) _array_index)) (Utilities|String|ToString(Object) (.texture (Utilities|Array|Get(acopy) (Variables|Default|GetDeck) _array_index))))) true true "(R=0.000000,G=0.660000,B=1.000000,A=1.000000)" 2e+02)))

(event Custom|PrintShuffledToScreen
  ;[0.15 0.1397 0.002652 0.5] Deck/Shuffle testing
  (for (_ _array_index) (Variables|Default|GetShuffledDeck)
    (Development|PrintString (Utilities|String|ToString(Text) (Utilities|Text|FormatText "Suit = {Suit}, Rank = {Rank}, Texture {Texture}" (Utilities|String|EnumtoString (.suit (Utilities|Array|Get(acopy) (Variables|Default|GetShuffledDeck) _array_index))) (.rank (Utilities|Array|Get(acopy) (Variables|Default|GetShuffledDeck) _array_index)) (Utilities|String|ToString(Object) (.texture (Utilities|Array|Get(acopy) (Variables|Default|GetShuffledDeck) _array_index))))) true true "(R=0.000000,G=0.660000,B=1.000000,A=1.000000)" 2e+02)))

(event EventBeginPlay
  (CallFunction|ClearDeck)
  (CallFunction|PopulateDeck)
  (CallFunction|ShuffleDeck))

(event Collision|EventActorBeginOverlap
  (params (OtherActor :type Actor%20Object%20Reference)))

(event EventTick
  (params (DeltaSeconds :type Float%20%28single-precision%29)))

(fn ConstructionScript)

(fn ClearDeck
  (Utilities|Array|Clear (Variables|Default|GetDeck)))

(fn CreateTextureNameString
  (params (Index :type Integer) (Index2 :type E_CardSuit%20Enum :default "NewEnumerator0"))
  (return (Utilities|String|ToString(Text) (Utilities|Text|FormatText "T_{Suit}_{Rank}" (Utilities|Select :Index Index2 :NewEnumerator0 "Hearts" :NewEnumerator1 "Diamonds" :NewEnumerator2 "Clubs" :NewEnumerator3 "Spades") (Utilities|Select :Index Index :Option%200 "" :Option%201 "1" :Option%202 "2" :Option%203 "3" :Option%204 "4" :Option%205 "5" :Option%206 "6" :Option%207 "7" :Option%208 "8" :Option%209 "9" :Option%2010 "10" :Option%2011 "11" :Option%2012 "12" :Option%2013 "13" :Option%2014 "14")))))

(fn PopulateDeck
  (bind _enumvalue (|ForEachE_CardSuit)
    (:LoopBody
      (for _index (range 1 13)
        (for _array_element (Variables|Default|GetCardTextures)
          (if (Utilities|Enum|Equal(Enum) (Utilities|GetObjectName _array_element) (CallFunction|CreateTextureNameString _index _enumvalue))
            (Utilities|Array|Add (Variables|Default|GetDeck) (Utilities|Struct|MakeST_CardStruct _enumvalue _index _array_element))))))
    (:then
      (Variables|Default|SetShuffledDeck (Variables|Default|GetDeck)))))

(fn ShuffleDeck
  (bind _shuffleddeck (Variables|Default|GetShuffledDeck))
  (bind _arrayindex (Utilities|Array|ReverseforEachLoop (Variables|Default|GetShuffledDeck))
    (:LoopBody
      (Variables|Default|SetCurrentShuffleIndex _arrayindex)
      (Variables|Default|SetRandomShuffleIndex (Math|Random|RandomIntegerinRange 0 (Variables|Default|GetCurrentShuffleIndex)))
      (Variables|Default|SetTempOriginal (Utilities|Array|Get(acopy) _shuffleddeck (Variables|Default|GetCurrentShuffleIndex)))
      (Variables|Default|SetTempRandom (Utilities|Array|Get(acopy) _shuffleddeck (Variables|Default|GetRandomShuffleIndex)))
      (Utilities|Array|SetArrayElem (Variables|Default|GetShuffledDeck) (Variables|Default|GetCurrentShuffleIndex) (Variables|Default|GetTempRandom) true)
      (Utilities|Array|SetArrayElem (Variables|Default|GetShuffledDeck) (Variables|Default|GetRandomShuffleIndex) (Variables|Default|GetTempOriginal) true))))

(fn DealPlayerCards
  (bind _shuffleddeck (Variables|Default|GetShuffledDeck))
  (bind _shuffleddeck_2 (Variables|Default|GetShuffledDeck))
  (bind _output (Utilities|Array|Get(acopy) _shuffleddeck))
  (bind _output_2 (Utilities|Array|Get(acopy) _shuffleddeck_2))
  (LocalVariables|SetCard_1_Temp _output)
  (Utilities|Array|RemoveItem (Variables|Default|GetShuffledDeck) _output)
  (LocalVariables|SetCard_2_Temp _output_2)
  (Utilities|Array|RemoveItem (Variables|Default|GetShuffledDeck) _output_2)
  (return (LocalVariables|GetCard_1_Temp) (LocalVariables|GetCard_2_Temp)))

(fn DealFlop
  (bind _shuffleddeck (Variables|Default|GetShuffledDeck))
  (bind _shuffleddeck_2 (Variables|Default|GetShuffledDeck))
  (bind _shuffleddeck_3 (Variables|Default|GetShuffledDeck))
  (bind _output (Utilities|Array|Get(acopy) _shuffleddeck))
  (bind _output_2 (Utilities|Array|Get(acopy) _shuffleddeck_2))
  (bind _output_3 (Utilities|Array|Get(acopy) _shuffleddeck_3))
  (LocalVariables|SetCard_1_Temp _output_2)
  (Utilities|Array|RemoveItem (Variables|Default|GetShuffledDeck) _output_2)
  (LocalVariables|SetCard_2_Temp _output)
  (Utilities|Array|RemoveItem (Variables|Default|GetShuffledDeck) _output)
  (LocalVariables|SetCard_3_Temp _output_3)
  (Utilities|Array|RemoveItem (Variables|Default|GetShuffledDeck) _output_3))

(fn DealTurn)

(fn DealRiver)

(fn Deal
  (LocalVariables|SetTempCard (Utilities|Array|Get(acopy) (Variables|Default|GetShuffledDeck)))
  (Utilities|Array|RemoveIndex (Variables|Default|GetShuffledDeck))
  (return (LocalVariables|GetTempCard)))
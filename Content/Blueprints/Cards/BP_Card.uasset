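; BP_Card is a card actor that displays a given texture on its Card component.
; SetCardTexture stores the texture, creates a dynamic instance of M_Card on the component's first material slot and sets its CardTexture parameter.
; BeginPlay calls SetCardTexture without supplying a texture, and each call creates a new material instance.
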(event EventBeginPlay
  (CallFunction|SetCardTexture))

(event Collision|EventActorBeginOverlap
  (params (OtherActor :type Actor%20Object%20Reference)))

(event EventTick
  (params (DeltaSeconds :type Float%20%28single-precision%29)))

(fn ConstructionScript)

(fn SetCardTexture
  (params (CardTexture :type Texture%202D%20Object%20Reference))
  ;[0.15 0.15 0.15 0.5] Set the texture of the card by creating a dynamic material instance and applying that to the cards material
  (Variables|Default|SetCardTexture CardTexture)
  (bind _returnvalue (Rendering|Material|CreateDynamicMaterialInstance (Variables|Default|GetCard) 0 "/Game/Assets/Textures/Cards/Materials/M_Card.M_Card" "None" :!class /Script/Engine.PrimitiveComponent))
  (bind _output_get (Variables|Default|SetDynamicCardMaterial _returnvalue))
  (Rendering|Material|SetMaterial (Variables|Default|GetCard) 0 _output_get)
  (Rendering|Material|SetTextureParameterValue (Variables|Default|GetDynamicCardMaterial) "CardTexture" (Variables|Default|GetCardTexture)))
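; Game mode for a poker game that sets up and runs a single deal when play begins.
; It gathers all BP_PokerPlayer actors, spawns a BP_Deck at the DeckSpawnPoint target point and shares it with BP_PokerGameState.
; Each player gets two cards, then the game state deals the flop.
; Hand evaluation is a stub: it appends community cards to each hand and assigns every player the same fixed rank.
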(event EventBeginPlay
  (CallFunction|StorePokerPlayers)
  (CallFunction|SpawnDeck)
  (bind _asbp_poker_game_state (Utilities|Casting|CastToBP_PokerGameState (Game|GetGameState)))
  (Variables|Default|SetPokerGameState _asbp_poker_game_state)
  (Variables|/Game/Blueprints/Game/BP_PokerGameState.BP_PokerGameState_C|SetDeckReference (Variables|Default|GetPokerGameState) (Variables|Default|GetGameDeck))
  (CallFunction|DealtoPlayers)
  (Default|DealFlop (Variables|Default|GetPokerGameState))
  (CallFunction|EvaluatePlayerHands))

(event EventTick
  (params (DeltaSeconds :type Float%20%28single-precision%29)))

(fn ConstructionScript)

(fn SpawnDeck
  (bind _outactors (Actor|GetAllActorsOfClass "/Script/Engine.TargetPoint"))
  (for _array_element _outactors
    (if (Utilities|Enum|Equal(Enum) (Utilities|GetDisplayName _array_element) "DeckSpawnPoint")
      (bind _returnvalue (Game|SpawnActorfromClass "/Game/Blueprints/Cards/BP_Deck.BP_Deck_C" (Math|Transform|MakeTransform (Transformation|GetActorLocation _array_element)) "Undefined" "MultiplyWithRoot" 0 0))
      (Variables|Default|SetGameDeck _returnvalue))))

(fn DealtoPlayers
  (for _array_element (Variables|Default|GetPokerPlayers)
    (for _index (range 0 1)
      (bind _dealtcard (Default|Deal (Variables|Default|GetGameDeck)))
      (Utilities|Array|Add (Variables|/Game/Blueprints/Player/BP_PokerPlayer.BP_PokerPlayer_C|GetHand _array_element) _dealtcard))))

(fn EvaluatePlayerHands
  (for (_array_element _array_index) (Variables|Default|GetPokerPlayers)
    (for _array_element_2 (Variables|/Game/Blueprints/Game/BP_PokerGameState.BP_PokerGameState_C|GetCommunityCards (Variables|Default|GetPokerGameState))
      (Utilities|Array|Add (Variables|/Game/Blueprints/Player/BP_PokerPlayer.BP_PokerPlayer_C|GetHand _array_element) _array_element_2))
    (Variables|/Game/Blueprints/Player/BP_PokerPlayer.BP_PokerPlayer_C|SetHandRank (Utilities|Array|Get(acopy) (Variables|Default|GetPokerPlayers) _array_index) "NewEnumerator5")))

(fn StorePokerPlayers
  (bind _outactors (Actor|GetAllActorsOfClass "/Game/Blueprints/Player/BP_PokerPlayer.BP_PokerPlayer_C"))
  (Variables|Default|SetPokerPlayers _outactors))
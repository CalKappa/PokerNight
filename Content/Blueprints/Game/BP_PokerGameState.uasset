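; Poker game state that holds the community cards and deals the flop.
; DealFlop moves the top three cards from the referenced deck's shuffled array into CommunityCards.
; It then finds level TargetPoints by display name, spawning a BP_Card at each of the three flop points with the matching card texture.
; DealTurn and DealRiver are empty stubs, and BeginPlay only calls its parent.
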(event EventBeginPlay
  (|CallParentFunction))

(event EventTick
  (params (DeltaSeconds :type Float%20%28single-precision%29)))

(fn ConstructionScript)

(fn DealFlop
  (for _index (range 0 2)
    (Utilities|Array|Add (Variables|Default|GetCommunityCards) (Utilities|Array|Get(acopy) (Variables|/Game/Blueprints/Cards/BP_Deck.BP_Deck_C|GetShuffledDeck (Variables|Default|GetDeckReference))))
    (Utilities|Array|RemoveIndex (Variables|/Game/Blueprints/Cards/BP_Deck.BP_Deck_C|GetShuffledDeck (Variables|Default|GetDeckReference))))
  (bind _outactors (Actor|GetAllActorsOfClass "/Script/Engine.TargetPoint"))
  (for _array_element _outactors
    (switch string (Utilities|GetDisplayName _array_element)
      (:FlopSpawnPoint_1
        (LocalVariables|SetCommunityCardIndexTemp 0))
      (:FlopSpawnPoint_2
        (LocalVariables|SetCommunityCardIndexTemp 1))
      (:FlopSpawnPoint_3
        (LocalVariables|SetCommunityCardIndexTemp 2)))
    (bind _returnvalue (Game|SpawnActorfromClass "/Game/Blueprints/Cards/BP_Card.BP_Card_C" (Math|Conversions|ToTransform(Vector) (Transformation|GetActorLocation _array_element)) "Undefined" "MultiplyWithRoot" 0 0))
    (Default|SetCardTexture _returnvalue (.texture (Utilities|Array|Get(acopy) (Variables|Default|GetCommunityCards) (LocalVariables|GetCommunityCardIndexTemp))))))

(fn DealTurn)

(fn DealRiver)